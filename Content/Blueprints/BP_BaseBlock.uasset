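; Voxel-style block terrain actor that the player can build on and dig into with the mouse.
; The construction script fills a Length by Width grid from four summed sine-product layers, putting below-zero heights in BlockD instances and the rest in Block.
; Clicks line-trace from the third-person follow camera: left adds a grid-snapped BlockD instance, right removes the hit index from Block if the hit actor matches it, otherwise from BlockD.
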(event `self.ReceiveBeginPlay`
  (`self.EnableInput` (`GameplayStatics.GetPlayerController` 0)))

(event `Key|LeftMouseButton`
  (params (Key :type "Key Structure"))
  (bind _returnvalue (`KismetMathLibrary.Conv_IntToDouble` (`self.TileSize`)))
  (:`Pressed`
    (bind _asbp_third_person_character (cast `/Game/ThirdPerson/Blueprints/BP_ThirdPersonCharacter` (`GameplayStatics.GetPlayerCharacter` 0)))
    (bind _followcamera (`/Game/ThirdPerson/Blueprints/BP_ThirdPersonCharacter.FollowCamera` _asbp_third_person_character))
    (bind _returnvalue_2 (`SceneComponent.K2_GetComponentLocation` _followcamera))
    (bind (_outhit _returnvalue_3) (`KismetSystemLibrary.LineTraceSingle` :`Start` _returnvalue_2 :`End` (+ _returnvalue_2 (* (`SceneComponent.GetForwardVector` _followcamera) 1000.0)) :`TraceChannel` "TraceTypeQuery1" :`DrawDebugType` "ForDuration" :`bIgnoreSelf` false))
    (bind (_bblockinghit _binitialoverlap _time _distance _location _impactpoint _normal _impactnormal _physmat _hitactor _hitcomponent _hitbonename _bonename _hititem _elementindex _faceindex _tracestart _traceend) (`GameplayStatics.BreakHitResult` _outhit))
    (`KismetSystemLibrary.PrintText` (`|FormatText` "loc: {loc} \nimpo: {imp} \nend: {end}" (`KismetStringLibrary.Conv_VectorToString` _location) (`KismetStringLibrary.Conv_VectorToString` _impactpoint) (`KismetStringLibrary.Conv_VectorToString` _traceend)))
    (`InstancedStaticMeshComponent.AddInstance` (`self.BlockD`) (`KismetMathLibrary.MakeTransform` (`KismetMathLibrary.MakeVector` (`KismetMathLibrary.GridSnap_Float` (.x (`KismetMathLibrary.SelectVector` _location _impactpoint _returnvalue_3)) _returnvalue) (`KismetMathLibrary.GridSnap_Float` (.y (`KismetMathLibrary.SelectVector` _location _impactpoint _returnvalue_3)) _returnvalue) (`KismetMathLibrary.GridSnap_Float` (.z (`KismetMathLibrary.SelectVector` _location _impactpoint _returnvalue_3)) _returnvalue))) false)))

(event `Key|RightMouseButton`
  (params (Key :type "Key Structure"))
  (:`Pressed`
    (bind _asbp_third_person_character (cast `/Game/ThirdPerson/Blueprints/BP_ThirdPersonCharacter` (`GameplayStatics.GetPlayerCharacter` 0)))
    (bind _followcamera (`/Game/ThirdPerson/Blueprints/BP_ThirdPersonCharacter.FollowCamera` _asbp_third_person_character))
    (bind _returnvalue (`SceneComponent.K2_GetComponentLocation` _followcamera))
    (bind _outhit (`KismetSystemLibrary.LineTraceSingle` :`Start` _returnvalue :`End` (+ _returnvalue (* (`SceneComponent.GetForwardVector` _followcamera) 1000.0)) :`TraceChannel` "TraceTypeQuery1" :`DrawDebugType` "ForDuration" :`bIgnoreSelf` false))
    (bind (_bblockinghit _binitialoverlap _time _distance _location _impactpoint _normal _impactnormal _physmat _hitactor _hitcomponent _hitbonename _bonename _hititem) (`GameplayStatics.BreakHitResult` _outhit))
    (if (== _hitactor (`self.Block`))
      (`InstancedStaticMeshComponent.RemoveInstance` (`self.Block`) _hititem)
      (else
        (`InstancedStaticMeshComponent.RemoveInstance` (`self.BlockD`) _hititem)))))

(fn `UserConstructionScript`
  (for _index (range 1 (+ (`self.Length`) 1))
    (for _index_2 (range 1 (+ (`self.Width`) 1))
      (bind _returnvalue (`KismetMathLibrary.Conv_IntToDouble` (* (`KismetMathLibrary.Round` (+ (* (`KismetMathLibrary.DegSin` (* _index_2 (`self.F1`))) (`KismetMathLibrary.DegSin` (* _index (`self.F1`))) (`self.H1`)) (* (`KismetMathLibrary.DegSin` (* _index_2 (`self.F2`))) (`KismetMathLibrary.DegSin` (* _index (`self.F2`))) (`self.H2`)) (* (`KismetMathLibrary.DegSin` (* (* _index_2 (`self.F3`)) 0.7)) (`KismetMathLibrary.DegSin` (* _index (`self.F3`))) (`self.H3`)) (* (`KismetMathLibrary.DegSin` (* _index_2 (`self.F4`))) (`KismetMathLibrary.DegSin` (* (* _index (`self.F4`)) 0.4)) (`self.H4`)))) (`self.TileSize`))))
      (if (< _returnvalue 0.0)
        (bind _returnvalue_2 (`KismetMathLibrary.Conv_VectorToTransform` (`KismetMathLibrary.MakeVector` (`KismetMathLibrary.Conv_IntToDouble` (* _index (`self.TileSize`))) (`KismetMathLibrary.Conv_IntToDouble` (* _index_2 (`self.TileSize`))) _returnvalue)))
        (`InstancedStaticMeshComponent.AddInstance` (`self.BlockD`) _returnvalue_2 false)
        (else
          (`InstancedStaticMeshComponent.AddInstance` (`self.Block`) _returnvalue_2 false))))))