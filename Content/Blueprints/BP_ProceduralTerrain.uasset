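; Procedural terrain actor that lets the player edit the terrain at runtime with mouse buttons and a key.
; It enables player input on BeginPlay, and each binding debug-draws a short line trace from the third-person character's follow camera.
; The hit location feeds terrain functions defined outside these graphs to raise, lower, level, add a tributary or simulate erosion.
; Trace results go unchecked, so edits fire even on a miss.
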(event `self.ReceiveBeginPlay`
  (`self.EnableInput` (`GameplayStatics.GetPlayerController` 0)))

(event `Key|LeftMouseButton`
  (params (Key :type "Key Structure"))
  (:`Pressed`
    (bind _asbp_third_person_character (cast `/Game/ThirdPerson/Blueprints/BP_ThirdPersonCharacter` (`GameplayStatics.GetPlayerCharacter` 0)))
    (bind _followcamera (`/Game/ThirdPerson/Blueprints/BP_ThirdPersonCharacter.FollowCamera` _asbp_third_person_character))
    (bind _returnvalue (`SceneComponent.K2_GetComponentLocation` _followcamera))
    (bind _outhit (`KismetSystemLibrary.LineTraceSingle` :`Start` _returnvalue :`End` (+ _returnvalue (* (`SceneComponent.GetForwardVector` _followcamera) 1000.0)) :`TraceChannel` "TraceTypeQuery1" :`DrawDebugType` "ForDuration" :`bIgnoreSelf` false))
    (`self.ModifyTerrainAt` (`.Location` (`GameplayStatics.BreakHitResult` _outhit)) 50.0 100.0)))

(event `Key|RightMouseButton`
  (params (Key :type "Key Structure"))
  (:`Pressed`
    (bind _asbp_third_person_character (cast `/Game/ThirdPerson/Blueprints/BP_ThirdPersonCharacter` (`GameplayStatics.GetPlayerCharacter` 0)))
    (bind _followcamera (`/Game/ThirdPerson/Blueprints/BP_ThirdPersonCharacter.FollowCamera` _asbp_third_person_character))
    (bind _returnvalue (`SceneComponent.K2_GetComponentLocation` _followcamera))
    (bind _outhit (`KismetSystemLibrary.LineTraceSingle` :`Start` _returnvalue :`End` (+ _returnvalue (* (`SceneComponent.GetForwardVector` _followcamera) 1000.0)) :`TraceChannel` "TraceTypeQuery1" :`DrawDebugType` "ForDuration" :`bIgnoreSelf` false))
    (`self.ModifyTerrainAt` (`.Location` (`GameplayStatics.BreakHitResult` _outhit)) 50.0 -100.0)))

(event `Key|ThumbMouseButton2`
  (params (Key :type "Key Structure"))
  (:`Pressed`
    (bind _asbp_third_person_character (cast `/Game/ThirdPerson/Blueprints/BP_ThirdPersonCharacter` (`GameplayStatics.GetPlayerCharacter` 0)))
    (bind _followcamera (`/Game/ThirdPerson/Blueprints/BP_ThirdPersonCharacter.FollowCamera` _asbp_third_person_character))
    (bind _returnvalue (`SceneComponent.K2_GetComponentLocation` _followcamera))
    (bind _outhit (`KismetSystemLibrary.LineTraceSingle` :`Start` _returnvalue :`End` (+ _returnvalue (* (`SceneComponent.GetForwardVector` _followcamera) 1000.0)) :`TraceChannel` "TraceTypeQuery1" :`DrawDebugType` "ForDuration" :`bIgnoreSelf` false))
    (`self.LevelTerrainAt` (`.Location` (`GameplayStatics.BreakHitResult` _outhit)) 500.0 -300.0)))

(event `Key|ThumbMouseButton`
  (params (Key :type "Key Structure"))
  (:`Pressed`
    (bind _asbp_third_person_character (cast `/Game/ThirdPerson/Blueprints/BP_ThirdPersonCharacter` (`GameplayStatics.GetPlayerCharacter` 0)))
    (bind _followcamera (`/Game/ThirdPerson/Blueprints/BP_ThirdPersonCharacter.FollowCamera` _asbp_third_person_character))
    (bind _returnvalue (`SceneComponent.K2_GetComponentLocation` _followcamera))
    (bind _outhit (`KismetSystemLibrary.LineTraceSingle` :`Start` _returnvalue :`End` (+ _returnvalue (* (`SceneComponent.GetForwardVector` _followcamera) 1000.0)) :`TraceChannel` "TraceTypeQuery1" :`DrawDebugType` "ForDuration" :`bIgnoreSelf` false))
    (`self.AddTributaryAt` (`.Location` (`GameplayStatics.BreakHitResult` _outhit)))))

(event `Key|One`
  (params (Key :type "Key Structure"))
  (:`Pressed`
    (bind _asbp_third_person_character (cast `/Game/ThirdPerson/Blueprints/BP_ThirdPersonCharacter` (`GameplayStatics.GetPlayerCharacter` 0)))
    (bind _followcamera (`/Game/ThirdPerson/Blueprints/BP_ThirdPersonCharacter.FollowCamera` _asbp_third_person_character))
    (bind _returnvalue (`SceneComponent.K2_GetComponentLocation` _followcamera))
    (bind _outhit (`KismetSystemLibrary.LineTraceSingle` :`Start` _returnvalue :`End` (+ _returnvalue (* (`SceneComponent.GetForwardVector` _followcamera) 1000.0)) :`TraceChannel` "TraceTypeQuery1" :`DrawDebugType` "ForDuration" :`bIgnoreSelf` false))
    (`self.SimulateErosionAt` (`.Location` (`GameplayStatics.BreakHitResult` _outhit)) 100.0 80 1.0 0.1)))

(fn `UserConstructionScript`)